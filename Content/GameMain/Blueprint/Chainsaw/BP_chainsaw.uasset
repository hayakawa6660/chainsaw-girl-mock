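; BP_chainsaw is a chainsaw Blueprint that tracks a gear number, shifted up and down from the keyboard.
; The U key calls GearUp while the gear is below its upper limit, and the D key calls GearDown while it is above zero.
; Each change prints the new gear to screen, and nothing else in the file uses the value yet.
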(event `Key|U`
  (params (Key :type "Key Structure"))
  (:`Pressed`
    (if (< (`self.gearNo`) 5)
      (`self.GearUp`))))

(event `Key|D`
  (params (Key :type "Key Structure"))
  (:`Pressed`
    (if (> (`self.gearNo`) 0)
      (`self.GearDown`))))

(fn `GearDown`
  (bind _output_get (set `self.gearNo` (- (`self.gearNo`) 1)))
  (`KismetSystemLibrary.PrintString` (`KismetStringLibrary.Conv_IntToString` _output_get)))

(fn `GearUp`
  (bind _output_get (set `self.gearNo` (+ (`self.gearNo`) 1)))
  (`KismetSystemLibrary.PrintString` (`KismetStringLibrary.Conv_IntToString` _output_get)))

(fn `UserConstructionScript`)