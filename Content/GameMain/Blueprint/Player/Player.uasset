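; Player character Blueprint, a thin child that configures behavior inherited from its parent class.
; On BeginPlay it calls Initialize with the attack stat, a named animation montage map, a Chainsaw2 weapon and a Player attack tag.
; Overlap, Tick and construction only forward to the parent, so this file adds no gameplay logic beyond that setup.
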(event `self.ReceiveBeginPlay`
  (`self.Initialize` (make `/Game/GameMain/Blueprint/Character/CharacterParameter` 100 10 0 (`|MakeMap` "Wait" "/Game/GameMain/Model/Marie3/Atimation/AttackMontage.AttackMontage" :!type "Name" :!valuetype "AnimMontage Object Reference")) (`|MakeArray` (`self.Chainsaw2`)) (`|MakeArray` "Player" :!type "Name")))

(event `self.ReceiveActorBeginOverlap`
  (params (OtherActor :type "Actor Object Reference"))
  (`parent.ReceiveActorBeginOverlap` OtherActor))

(event `self.ReceiveTick`
  (params (DeltaSeconds :type "Float (single-precision)"))
  (`parent.ReceiveTick` DeltaSeconds))

(fn `UserConstructionScript`
  (`parent.UserConstructionScript`))