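; Player character that moves on the control-yaw plane, attacks with a child-actor chainsaw and shifts its gears.
; Attack montage playback blocks movement, and a named montage section enables chainsaw collision, shaking the camera while enemies overlap.
; Energy serves as health, draining each tick by gear rate, dropping on damage and feeding the game mode's UI actor.
; Drain and post-hit invincibility count frames assuming 60 fps, ignoring delta time.
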(event `self.ReceiveTick`
  (params (DeltaSeconds :type "Float (single-precision)"))
  (bind _animinstance (`self.animInstance`))
  (bind _returnvalue (`AnimInstance.GetCurrentActiveMontage` _animinstance))
  (`|ExecutionSequence`
    (:`then_0`
      (`self.EnergyConsumptionCalcu`)
      (`self.AttackShakeCamera`))
    (:`then_1`
      (if (`self.isInvincible`)
        (`self.UpdateInvincibleCount`)))
    (:`then_2`
      ;[1 1 1] Attack
      (bind _output_get (set `self.isAttack` (`AnimInstance.Montage_IsPlaying` _animinstance _returnvalue)))
      (bind _output_get_2 (set `self.onAttack` (and _output_get (== (`AnimInstance.Montage_GetCurrentSection` (`self.animInstance`) _returnvalue) (`self.onAttackCollisionName`)))))
      (`/Game/GameMain/Blueprint/Chainsaw/BP_chainsaw.SetCollisionEnable` (`self.As BP Chainsaw`) _output_get_2))))

(event `InputAction|Attack`
  (params (Key :type "Key Structure"))
  ;[1 1 1] Attack
  (:`Pressed`
    (`AnimInstance.Montage_Play` (`self.animInstance`) "/Game/GameMain/Model/Marie3/Atimation/AttackMontage.AttackMontage" 1.0 "Duration" 0.0 true)))

(event `self.ReceiveBeginPlay`
  ;[1 1 1] Initialize
  (`self.Initialize`))

(event `InputAction|GearUp`
  (params (Key :type "Key Structure"))
  ;[1 1 1] Gear
  (:`Pressed`
    (if (not (`self.isSetGear`))
      (`/Game/GameMain/Blueprint/Chainsaw/BP_chainsaw.GearUp` (`self.As BP Chainsaw`))
      (set `self.isSetGear` true)))
  (:`Released`
    (set `self.isSetGear` false)))

(event `InputAxis|Forward`
  (params (AxisValue :type "Float (single-precision)"))
  ;[1 1 1] 移動処理
  (if (not (`self.isAttack`))
    (`self.AddMovementInput` (`KismetMathLibrary.GetForwardVector` (`KismetMathLibrary.MakeRotator` 0.0 0.0 (.yaw (`self.GetControlRotation`)))) AxisValue)))

(event `InputAction|GearDown`
  (params (Key :type "Key Structure"))
  ;[1 1 1] Gear
  (:`Pressed`
    (if (not (`self.isSetGear`))
      (`/Game/GameMain/Blueprint/Chainsaw/BP_chainsaw.GearDown` (`self.As BP Chainsaw`))
      (set `self.isSetGear` true)))
  (:`Released`
    (set `self.isSetGear` false)))

(event `InputAxis|Right`
  (params (AxisValue :type "Float (single-precision)"))
  ;[1 1 1] 移動処理
  (if (not (`self.isAttack`))
    (`self.AddMovementInput` (`KismetMathLibrary.GetRightVector` (`KismetMathLibrary.MakeRotator` 0.0 0.0 (.yaw (`self.GetControlRotation`)))) AxisValue)))

(fn `AttackCameraShake`
  (`GameplayStatics.PlayWorldCameraShake` "/Game/GameMain/Blueprint/Camera/AttackCameraShake.AttackCameraShake_C" (`self.K2_GetActorLocation`) 0.0 2000.0))

(fn `AttackShakeCamera`
  ;[1 1 1] Attack Shake Camera
  (for _array_element (`PrimitiveComponent.GetOverlappingActors` (`/Game/GameMain/Blueprint/Chainsaw/BP_chainsaw.Capsule` (`self.As BP Chainsaw`)) "/Game/GameMain/Blueprint/Enemy/AI/Enemy_Character.Enemy_Character_C")
    (`/Engine/EditorBlueprintResources/StandardMacros.IsValid` _array_element
      (:`Is Valid`
        (if (`self.onAttack`)
          (`self.AttackCameraShake`))))))

(fn `EnergyConsumptionCalcu`
  (bind _resultrate (`/Game/GameMain/Blueprint/Chainsaw/BP_chainsaw.GetCurrentGearRate` (`self.As BP Chainsaw`)))
  (bind _output_get (set `self.energy` (`KismetMathLibrary.FMax` (- (`self.energy`) (* _resultrate (/ (`self.maxEnergy`) (* (`self.energyConsumptionTime`) 60.0)))))))
  (`/Game/GameMain/UI/TestUI.SetEnergy` (`self.UIActor`) (/ _output_get (`self.maxEnergy`))))

(fn `Initialize`
  (`|ExecutionSequence`
    (:`then_0`
      (bind _asbp_chainsaw (cast `/Game/GameMain/Blueprint/Chainsaw/BP_chainsaw` (`ChildActorComponent.ChildActor` (`self.BP_chainsaw`))))
      (set `self.As BP Chainsaw` _asbp_chainsaw)
      (set `self.animInstance` (`SkeletalMeshComponent.GetAnimInstance` (`self.Mesh`)))
      (set `self.energy` (`self.maxEnergy`))
      (bind _aschainsaw_girl_game (cast `/Game/GameMain/Blueprint/GameMode/ChainsawGirlGame` (`GameplayStatics.GetGameMode`)))
      (set `self.UIActor` (`/Game/GameMain/Blueprint/GameMode/ChainsawGirlGame.UIActor` _aschainsaw_girl_game)))))

(fn `SetInvincible`
  (params (invincibleTime :type "Float (double-precision)"))
  (set `self.invincibleCounter` (* invincibleTime 60.0))
  (set `self.isInvincible` true))

(fn `TakeDamage`
  (params (damage :type Integer))
  (if (not (`self.isInvincible`))
    (set `self.energy` (- (`self.energy`) damage))
    (`self.SetInvincible` 2.0)))

(fn `UpdateInvincibleCount`
  (`/Engine/EditorBlueprintResources/StandardMacros.DecrementFloat` (`self.invincibleCounter`)
    (:`  `
      (if (< (`self.invincibleCounter`) 0.0)
        (set `self.isInvincible` false)))))

(fn `UserConstructionScript`)