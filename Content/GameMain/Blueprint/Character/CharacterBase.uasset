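; CharacterBase is the shared character Blueprint that handles health, death state, tag-filtered attacks and animation playback.
; Initialize takes a character info struct, target tags and weapon child actors, sets HP, caches the AnimInstance and passes itself to each WeaponBase.
; AttackChara applies the character's attack value through TakeDamage when the hit character carries a target tag.
; PlayAnimation looks up montages by key in the info's map, skipping requests while the current one plays.
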(fn `AttackChara`
  (params (hitCharacter :type "/Game/GameMain/Blueprint/Character/CharacterBase Object Reference"))
  (locals (hitChara :type "/Game/GameMain/Blueprint/Character/CharacterBase Object Reference"))
  (bind (_charainfo_hitpoint _charainfo_atk) (break `/Game/GameMain/Blueprint/Character/CharacterParameter` (`self.charaInfo`)))
  (set `local.hitChara` hitCharacter)
  ;[1 1 1] タグチェック
  (for _array_element (`self.attackPartnerTag`)
    (if (!= (`KismetArrayLibrary.Array_Find` (`Actor.Tags` (`local.hitChara`)) _array_element) -1)
      ;[1 1 1] 相手にダメージ
      (`self.TakeDamage` (`local.hitChara`) _charainfo_atk)
      (break))))

(fn `GetCharacterParam`
  (returns (CharaInfo :type "/Game/GameMain/Blueprint/Character/CharacterParameter Structure"))
  (return (`self.charaInfo`)))

(fn `GetIsDead`
  (returns (isDead :type Boolean))
  (return (`self.isDead`)))

(fn `Initialize`
  (params (CharaInfo :type "/Game/GameMain/Blueprint/Character/CharacterParameter Structure") (Weapons :type "Array of ChildActorComponent Object Reference") (attackCharaTag :type "Array of Name"))
  (locals (needInitWeapons :type "Array of ChildActorComponent Object Reference"))
  (bind _charainfo_hitpoint (break `/Game/GameMain/Blueprint/Character/CharacterParameter` (`self.charaInfo`)))
  (set `self.charaInfo` CharaInfo)
  (set `local.needInitWeapons` Weapons)
  (set `self.attackPartnerTag` attackCharaTag)
  (`|ExecutionSequence`
    (:`then_0`
      ;[1 1 1] HPの最大値設定
      (set `self.currentHp` _charainfo_hitpoint))
    (:`then_1`
      ;[1 1 1] アニメーションインスタンスを取得
      (set `self.animInstance` (`SkeletalMeshComponent.GetAnimInstance` (`self.Mesh`))))
    (:`then_2`
      ;[1 1 1] 武器クラス初期化
      (for _array_element (`local.needInitWeapons`)
        (bind _asweapon_base (cast `/Game/GameMain/Blueprint/Character/WeaponBase` (`ChildActorComponent.ChildActor` _array_element)))
        (`/Game/GameMain/Blueprint/Character/WeaponBase.Initialize` _asweapon_base self)))))

(fn `PlayAnimation`
  (params (setAnimKey :type Name) (resetMontage :type Boolean))
  (bind (_charainfo_hitpoint _charainfo_atk _charainfo_def _charainfo_animations) (break `/Game/GameMain/Blueprint/Character/CharacterParameter` (`self.charaInfo`)))
  (bind (_value _returnvalue) (`BlueprintMapLibrary.Map_Find` _charainfo_animations setAnimKey))
  (if (not (`AnimInstance.Montage_IsPlaying` (`self.animInstance`) (`self.currentAnim`)))
    (`/Engine/EditorBlueprintResources/StandardMacros.IsValid` (`self.animInstance`)
      (:`Is Valid`
        (if _returnvalue
          (`AnimInstance.Montage_Play` (`self.animInstance`) _value 1.0 "MontageLength" 0.0 true)
          (set `self.currentAnim` _value)
          (else
            ;[1 1 1] アニメーションがmap内に存在しない
            (`KismetSystemLibrary.PrintString` (`KismetStringLibrary.Concat_StrStr` (`KismetStringLibrary.Conv_NameToString` setAnimKey) "というアニメーションは登録されていません")))))
      (:`Is Not Valid`
        (`KismetSystemLibrary.PrintString` "アニメーションインスタンスがnullです")))))

(fn `SetAttackTag`
  (params (setTags :type "Array of Name"))
  (set `self.attackPartnerTag` setTags))

(fn `TakeDamage`
  (params (damage :type Integer))
  (bind _returnvalue (- (`self.currentHp`) damage))
  (bind _returnvalue_2 (`KismetMathLibrary.SelectInt` _returnvalue 0 (> _returnvalue 0)))
  (bind _output_get (set `self.currentHp` _returnvalue_2))
  (set `self.isDead` (== _returnvalue_2 0))
  (`KismetSystemLibrary.PrintString` (`KismetStringLibrary.Conv_IntToString` _output_get)))

(fn `UserConstructionScript`)