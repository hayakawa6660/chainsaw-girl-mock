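; AI controller for enemies that runs the BT_Enemy behavior tree on possession and feeds it perception results.
; When AI Perception updates, a successfully sensed actor tagged Player is passed to Tracking; any other update passes no target.
; Tracking writes that target, or empty, to the EnemyActor blackboard key and sets HasLineofSight to false in both cases.
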(event `self.ReceivePossess`
  (params (PossessedPawn :type "Pawn Object Reference"))
  (`self.RunBehaviorTree` "/Game/GameMain/Blueprint/Enemy/BT_Enemy.BT_Enemy"))

(event `self.AIPerception.OnTargetPerceptionUpdated`
  (params (Actor :type "Actor Object Reference") (Stimulus :type "AIStimulus Structure"))
  (bind _output_get (set `self.target` Actor))
  (if (and (`self.ActorHasTag` _output_get "Player") (`.bSuccessfullySensed` (break `AIStimulus` Stimulus)))
    (`self.Tracking` (`self.target`))
    (else
      (`self.Tracking` null))))

(fn `Tracking`
  (params (targetActor :type "Actor Object Reference"))
  (`BlackboardComponent.SetValueAsBool` (`self.Blackboard`) (`self.HasLineofSight`) false)
  (`BlackboardComponent.SetValueAsObject` (`self.Blackboard`) (`self.enemyActor`) targetActor))

(fn `UserConstructionScript`)